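; Paper2D portal actor that teleports the player character to set X and Z coordinates when the player overlaps its box trigger.
; A DoOnce gate blocks retriggering while the sprite swaps, waits a delay and swaps again, then the ResetTrampoline event reopens it.
; Tick is empty, and a leftover overlap debug print is never run.
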(event `self.ReceiveBeginPlay`
  (`parent.ReceiveBeginPlay`))

(event `self.ReceiveTick`
  (params (DeltaSeconds :type "Float (single-precision)")))

(event `self.Box.OnComponentBeginOverlap`
  (params (OverlappedComponent :type "PrimitiveComponent Object Reference") (OtherActor :type "Actor Object Reference") (OtherComp :type "PrimitiveComponent Object Reference") (OtherBodyIndex :type Integer) (bFromSweep :type Boolean) (SweepResult :type "HitResult Structure (by ref)"))
  (if (== OtherActor (`self.Playercharacterref`))
    (`/Engine/EditorBlueprintResources/StandardMacros.DoOnce` false :!label _label
      (:`Completed`
        (`self.K2_TeleportTo` :`self` (`self.Playercharacterref`) :`DestLocation` (`KismetMathLibrary.MakeVector` (`self.Coordinates X`) 0.0 (`self.Coordinates Z`)))
        (`PaperSpriteComponent.SetSprite` (`self.PaperSprite`) "/Game/Assets/portal_anim/portal_anim1_Sprite.portal_anim1_Sprite")
        (`KismetSystemLibrary.Delay` (`self.Duration`))
        (`PaperSpriteComponent.SetSprite` (`self.PaperSprite`) "/Game/Assets/portal_anim/portal_anim2_Sprite.portal_anim2_Sprite")
        (`self.Reset trampoline`)))))

(event `Reset trampoline`
  (goto _label :!via `Reset`))

(fn `UserConstructionScript`
  (`parent.UserConstructionScript`))